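; Enemy character for a top-down game, driven by an EnemyController that receives its patrol waypoints on BeginPlay when WaypointFrom is set.
; PawnSensing reports the player as visible, and a retriggerable delay clears that flag shortly after sightings stop.
; Hitting a slamming Door breaks it, ragdolls the enemy and destroys its controller, then plays a brief slow-motion hit with a player camera zoom.
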(event OnSeePawn(PawnSensing)
  (params (Pawn :type Pawn%20Object%20Reference))
  (Default|EventPlayerVisible (Variables|Default|GetEnemyController) true)
  (Utilities|FlowControl|RetriggerableDelay 0.2)
  (Default|EventPlayerVisible (Variables|Default|GetEnemyController) false))

(event OnComponentHit(CapsuleComponent)
  (params (HitComponent :type Primitive%20Component%20Object%20Reference) (OtherActor :type Actor%20Object%20Reference) (OtherComp :type Primitive%20Component%20Object%20Reference) (NormalImpulse :type Vector :default "0, 0, 0") (Hit :type Hit%20Result%20Structure%20%28by%20ref%29))
  (bind _asdoor (Utilities|Casting|CastToDoor OtherActor))
  (if (Variables|/Game/Blueprints/Door.Door_C|GetSlamming _asdoor)
    (Default|Break _asdoor)
    (Collision|SetCollisionEnabled (Variables|Character|GetMesh) "QueryAndPhysics")
    (Physics|SetSimulatePhysics (Variables|Character|GetMesh) true)
    (Collision|SetCollisionEnabled (Variables|Collision|GetCapsuleComponent) "NoCollision")
    (Actor|DestroyActor (Variables|Default|GetEnemyController))
    (bind _astop_down_character (Utilities|Casting|CastToTopDownCharacter (Game|Player|GetPlayerPawn 0)))
    (Variables|/Game/Blueprints/TopDownCharacter.TopDownCharacter_C|SetzoomIn _astop_down_character true)
    (Utilities|FlowControl|Delay 0.1)
    (Utilities|Time|SetGlobalTimeDilation 0.1)
    (Utilities|FlowControl|Delay 0.2)
    (Utilities|Time|SetGlobalTimeDilation 1.0)
    (Variables|/Game/Blueprints/TopDownCharacter.TopDownCharacter_C|SetzoomIn _astop_down_character false)))

(event EventBeginPlay
  (bind _asenemy_controller (Utilities|Casting|CastToEnemyController (AI|GetAIController self)))
  (Variables|Default|SetEnemyController _asenemy_controller)
  (if (!= (Math|Vector|VectorLengthSquared (Variables|Default|GetWaypointFrom)) 0.0)
    (Default|EventSetWaypoints (Variables|Default|GetEnemyController) (Variables|Default|GetWaypointFrom) (Variables|Default|GetWaypointTo))))

(fn ConstructionScript)