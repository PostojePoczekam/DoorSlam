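; EnemyController is an AI controller that drives an enemy through a behavior tree and feeds it information about the player.
; On BeginPlay it sets up the enemy blackboard, stores player pawn 0 as the target actor and runs the tree.
; A PlayerVisible event writes the visibility flag and records the player's current location as last known, whether visibility is true or false.
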(event Custom|Event%20PlayerVisible
  (params (visible :type Boolean))
  (AI|Components|Blackboard|SetValueasBool (Variables|Default|GetEnemyBlackboard) (Variables|Default|GetPlayerVisibleName) visible)
  (AI|Components|Blackboard|SetValueasVector (Variables|Default|GetEnemyBlackboard) (Variables|Default|GetLastPlayerLocationName) (Transformation|GetActorLocation (Game|Player|GetPlayerPawn 0))))

(event EventBeginPlay
  (bind _blackboardcomponent (Class|AIController|UseBlackboard "/Game/Blueprints/Enemy/EnemyBlackboard.EnemyBlackboard"))
  (bind _output_get (Variables|Default|SetEnemyBlackboard _blackboardcomponent))
  (AI|Components|Blackboard|SetValueasObject _output_get (Variables|Default|GetPlayerActorName) (Game|Player|GetPlayerPawn 0))
  (AI|RunBehaviorTree "/Game/Blueprints/Enemy/EnemyBehaviorTree.EnemyBehaviorTree"))

(fn ConstructionScript)